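; Projectile Blueprint that flies forward, damages obstacles and walls, and expires after a set lifetime.
; Tick offsets it along local forward by Speed per frame, unscaled by delta time and without sweep, while counting Lifetime down to destruction.
; On overlap, the bullet destroys itself, decrements Health on an obstacle or Wall, and destroys any other actor outright.
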(event OnComponentBeginOverlap(bullet)
  (params (OverlappedComponent :type Primitive%20Component%20Object%20Reference) (OtherActor :type Actor%20Object%20Reference) (OtherComp :type Primitive%20Component%20Object%20Reference) (OtherBodyIndex :type Integer) (bFromSweep :type Boolean) (SweepResult :type Hit%20Result%20Structure%20%28by%20ref%29))
  (Actor|DestroyActor)
  (bind _asobstacle (Utilities|Casting|CastToobstacle OtherActor)
    (:then
      (Variables|/Game/blueprints/obstacle.obstacle_C|SetHealth _asobstacle (- (Variables|/Game/blueprints/obstacle.obstacle_C|GetHealth _asobstacle) 1)))
    (:CastFailed
      (bind _aswall (Utilities|Casting|CastToWall OtherActor)
        (:then
          (Variables|/Game/blueprints/Wall.Wall_C|Sethealth _aswall (- (Variables|/Game/blueprints/Wall.Wall_C|Gethealth _aswall) 1)))
        (:CastFailed
          (Actor|DestroyActor OtherActor))))))

(event EventBeginPlay)

(event Collision|EventActorBeginOverlap
  (params (OtherActor :type Actor%20Object%20Reference)))

(event EventTick
  (params (DeltaSeconds :type Float%20%28single-precision%29))
  (Transformation|AddActorLocalOffset (* (Class|KismetMathLibrary|VectorForward) (Variables|Default|Getspeed)) false false)
  (Variables|Default|Setlifetime (- (Variables|Default|Getlifetime) DeltaSeconds))
  (if (not (> (Variables|Default|Getlifetime) 0.0))
    (Actor|DestroyActor)))

(fn ConstructionScript)
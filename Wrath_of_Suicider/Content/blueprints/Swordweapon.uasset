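; Sword weapon actor that spins for a limited lifetime and destroys whatever actor it touches.
; Tick rotates StaticMesh1 by a fixed step each frame, independent of frame rate scaling, and counts Lifetime down by delta seconds, destroying the sword when it runs out.
; An overlap on StaticMesh destroys both the sword and the other actor, with no filtering or damage step.
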(event OnComponentBeginOverlap(StaticMesh)
  (params (OverlappedComponent :type Primitive%20Component%20Object%20Reference) (OtherActor :type Actor%20Object%20Reference) (OtherComp :type Primitive%20Component%20Object%20Reference) (OtherBodyIndex :type Integer) (bFromSweep :type Boolean) (SweepResult :type Hit%20Result%20Structure%20%28by%20ref%29))
  (Actor|DestroyActor)
  (Actor|DestroyActor OtherActor))

(event EventBeginPlay)

(event Collision|EventActorBeginOverlap
  (params (OtherActor :type Actor%20Object%20Reference)))

(event EventTick
  (params (DeltaSeconds :type Float%20%28single-precision%29))
  (Transformation|AddLocalRotation (Variables|Default|GetStaticMesh1) "0,6.000000, 0" false false)
  (Variables|Default|Setlifetime (- (Variables|Default|Getlifetime) (Utilities|Time|GetWorldDeltaSeconds)))
  (if (not (> (Variables|Default|Getlifetime) 0.0))
    (Actor|DestroyActor)))

(fn ConstructionScript)
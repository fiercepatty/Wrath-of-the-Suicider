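; Destructible obstacle actor that breaks apart into smaller pieces once its Health drops below zero.
; Tick polls Health, then three nested loops spawn half-scale Pieces actors in an evenly spaced 3D grid from the actor's location.
; DestroyActor is called inside the innermost loop after each spawn attempt, rather than once after the loops finish.
; Nothing in this graph changes Health.
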(event EventBeginPlay)

(event Collision|EventActorBeginOverlap
  (params (OtherActor :type Actor%20Object%20Reference)))

(event EventTick
  (params (DeltaSeconds :type Float%20%28single-precision%29))
  (bind _returnvalue (Transformation|GetActorLocation))
  (bind (_x _y _z) (Math|Vector|BreakVector _returnvalue))
  (if (< (Variables|Default|GetHealth) 0)
    (for _index (range 0 3)
      (for _index_2 (range 0 3)
        (for _index_3 (range 0 3)
          (Game|SpawnActorfromClass "/Game/blueprints/Pieces.Pieces_C" (Math|Transform|MakeTransform (Math|Vector|MakeVector (+ _x (* _index 6e+01)) (+ _y (* _index_2 6e+01)) (+ (* _index_3 6e+01) _z)) "0, 0, 0" "0.500000,0.500000,0.500000") "AdjustIfPossibleButDontSpawnIfColliding" 0 0)
          (Actor|DestroyActor))))))

(fn ConstructionScript)